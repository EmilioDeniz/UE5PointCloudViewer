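; HUD for the point cloud viewer that adds the HUD widget and provides drag-rectangle selection of cloud points.
; Crop press and release store corrected cursor trace hits as opposite corners, while DrawHUD draws the rectangle during the drag.
; On release, temporary sphere and cube actors define the box used to select or deselect points, per the controller's DeselectMode.
; The resulting selection is dispatched through the widget's editor reference.
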(event `self.ReceiveBeginPlay`
  (bind _returnvalue (`|CreateWidget` "/Game/Blueprints/CloudViewHUDWidgetBlueprint.CloudViewHUDWidgetBlueprint_C"))
  (bind _output_get (set `self.HUD_Ref` _returnvalue))
  (`UserWidget.AddToViewport` _output_get 0))

(event `/Game/Blueprints/SelectionInterface.Crop Pressed`
  (bind (_locationx _locationy) (`PlayerController.GetMousePosition` (`GameplayStatics.GetPlayerController` 0)))
  (bind _returnvalue (`GameplayStatics.GetActorOfClass` "/Game/PointCloudActorBlueprint.PointCloudActorBlueprint_C"))
  (set `self.ActorRef` _returnvalue)
  (set `self.IsDrawing` true)
  (bind _output_get (set `self.MouseStartPos` (`KismetMathLibrary.MakeVector2D` _locationx _locationy)))
  (set `self.MouseCurrentPos` _output_get)
  (bind _returnvalue_2 (`CloudEditorUtils.CalculateCorrectHitPoint` (`self.GetTransform` (`self.ActorRef`)) (`.Location` (`GameplayStatics.BreakHitResult` (`PlayerController.GetHitResultUnderCursorByChannel` (`GameplayStatics.GetPlayerController` 0) "TraceTypeQuery3" true)))))
  (set `self.StartLocation` _returnvalue_2))

(event `/Game/Blueprints/SelectionInterface.Crop Held`
  (bind (_locationx _locationy) (`PlayerController.GetMousePosition` (`GameplayStatics.GetPlayerController` 0)))
  (set `self.MouseCurrentPos` (`KismetMathLibrary.MakeVector2D` _locationx _locationy)))

(event `/Game/Blueprints/SelectionInterface.Crop Released`
  (set `self.IsDrawing` false)
  (bind _returnvalue (`CloudEditorUtils.CalculateCorrectHitPoint` (`self.GetTransform` (`self.ActorRef`)) (`.Location` (`GameplayStatics.BreakHitResult` (`PlayerController.GetHitResultUnderCursorByChannel` (`GameplayStatics.GetPlayerController` 0) "TraceTypeQuery3" true)))))
  (bind _output_get (set `self.EndLocation` _returnvalue))
  (set `self.MiddlePoint` (/ (+ _output_get (`self.StartLocation`)) 2))
  (bind _asmouse_player_controller (cast `/Game/MousePlayerController` (`GameplayStatics.GetPlayerController` 0)))
  (set `/Game/MousePlayerController.SelectPointsMode` false _asmouse_player_controller)
  (bind _aspoint_cloud_component (cast `PointCloudComponent` (`LidarPointCloudActor.PointCloudComponent` (`self.ActorRef`))))
  (`self.Get Points` _aspoint_cloud_component (`self.Reference Points`)))

(event `self.ReceiveDrawHUD`
  (params (SizeX :type Integer) (SizeY :type Integer))
  (bind (_mousestartpos_x _mousestartpos_y) (`KismetMathLibrary.BreakVector2D` (`self.MouseStartPos`)))
  (bind (_mousecurrentpos_x _mousecurrentpos_y) (`KismetMathLibrary.BreakVector2D` (`self.MouseCurrentPos`)))
  (if (`self.IsDrawing`)
    (`self.DrawRect` (struct :`R` 1.0 :`G` 0.188499 :`A` 0.513) _mousestartpos_x _mousestartpos_y (- _mousecurrentpos_x _mousestartpos_x) (- _mousecurrentpos_y _mousestartpos_y))))

(fn `Get Points`
  (params (ComponentRef :type "PointCloudComponent Object Reference") (TargetArray :type "Array of Vector Structure (by ref)"))
  (bind _pointcloudref (`self.PointCloudRef`))
  (bind _reference_points (`self.Reference Points`))
  (set `self.PointCloudRef` ComponentRef)
  (`|ExecutionSequence`
    (:`then_0`
      (bind _returnvalue (`|SpawnActorFromClass` "/Game/Blueprints/CoordinateSphereBlueprint.CoordinateSphereBlueprint_C" (`KismetMathLibrary.Conv_VectorToTransform` (`self.StartLocation`)) "Undefined" "MultiplyWithRoot" (`self.ActorRef`) false null))
      (bind _returnvalue_2 (`|SpawnActorFromClass` "/Game/Blueprints/CoordinateSphereBlueprint.CoordinateSphereBlueprint_C" (`KismetMathLibrary.Conv_VectorToTransform` (`self.EndLocation`)) "Undefined" "MultiplyWithRoot" (`self.ActorRef`) false null)))
    (:`then_1`
      (`KismetArrayLibrary.Array_Add` _reference_points (`self.K2_GetActorLocation` _returnvalue))
      (`KismetArrayLibrary.Array_Add` _reference_points (`self.K2_GetActorLocation` _returnvalue_2)))
    (:`then_2`
      (bind _returnvalue_3 (`|SpawnActorFromClass` "/Game/Blueprints/SelectCubeActorBlueprint.SelectCubeActorBlueprint_C" (`KismetMathLibrary.Conv_VectorToTransform` (`self.MiddlePoint`)) "Undefined" "MultiplyWithRoot" (`self.ActorRef`) false (`self.Reference Points`) null))
      (`PointCloudComponent.SetPointList` _pointcloudref)
      (bind _returnvalue_4 (`PointCloudComponent.GetStartingBox` _pointcloudref _returnvalue_3))
      (bind _returnvalue_5 (`PointCloudComponent.GetCenter` _pointcloudref _returnvalue_3))
      (`self.K2_DestroyActor` _returnvalue_3)
      (`self.K2_DestroyActor` _returnvalue)
      (`self.K2_DestroyActor` _returnvalue_2)
      (bind _asmouse_player_controller (cast `/Game/MousePlayerController` (`GameplayStatics.GetPlayerController` 0)))
      (if (`/Game/MousePlayerController.DeselectMode` _asmouse_player_controller)
        (`PointCloudComponent.DeselectPoints` (`self.PointCloudRef`) _returnvalue_5 _returnvalue_4)
        (else
          (`PointCloudComponent.SelectPoints` (`self.PointCloudRef`) _returnvalue_5 _returnvalue_4)))
      (`KismetArrayLibrary.Array_Clear` (`self.Reference Points`))
      (`/Game/Blueprints/EditPointCloudHUDBlueprint.PointsSelectedDispatcher` (`/Game/Blueprints/CloudViewHUDWidgetBlueprint.EditorRef` (`self.HUD_Ref`)) (`PointCloudComponent.bPointsSelected` (`self.PointCloudRef`))))))

(fn `UserConstructionScript`)